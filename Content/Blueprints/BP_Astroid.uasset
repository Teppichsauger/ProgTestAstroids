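; BP_Astroid is an asteroid actor that flashes its emissive material when its mesh is hit.
; On begin play it creates a dynamic material instance for the first material slot of the mesh.
; Each component hit calls OnHit with the other actor, then restarts the Blink timeline at raised speed to drive the material's "Emmisive" parameter.
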(event OnComponentHit(AstroidMesh)
  (params (HitComponent :type Primitive%20Component%20Object%20Reference) (OtherActor :type Actor%20Object%20Reference) (OtherComp :type Primitive%20Component%20Object%20Reference) (NormalImpulse :type Vector :default "0, 0, 0") (Hit :type Hit%20Result%20Structure%20%28by%20ref%29))
  (Utilities|FlowControl|Sequence
    (:then_0
      (Class|Astroid|OnHit OtherActor))
    (:then_1
      (Utilities|IsValid (Variables|Default|GetBlink)
        (:Is%20Valid
          (Components|Timeline|SetPlayRate (Variables|Default|GetBlink) 5.0)
          (bind _alpha (Timeline|Blink PlayFromStart)
            (:Update
              (Rendering|Material|SetScalarParameterValue (Variables|Default|GetAstroid_DynMat) "Emmisive" _alpha :!class /Script/Engine.MaterialInstanceDynamic)
              (Rendering|Material|SetMaterial (Variables|Default|GetAstroidMesh) 0 (Variables|Default|GetAstroid_DynMat)))))))))

(event EventBeginPlay
  (bind _astroidmesh (Variables|Default|GetAstroidMesh))
  (bind _returnvalue (Rendering|Material|CreateDynamicMaterialInstance _astroidmesh 0 (Rendering|Material|GetMaterial _astroidmesh 0) "None" :!class /Script/Engine.PrimitiveComponent))
  (bind _output_get (Variables|Default|SetAstroid_DynMat _returnvalue))
  (Rendering|Material|SetMaterial (Variables|Default|GetAstroidMesh) 0 _output_get))

(fn ConstructionScript)