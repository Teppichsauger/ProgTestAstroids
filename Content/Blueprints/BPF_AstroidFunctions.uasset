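; Blueprint function library for the Asteroids game that exposes player ship and score values through three getter functions.
; Force field strength is read from the player pawn's BP_SpaceShip and remapped with a clamped range into a rounded percentage.
; The ammunition getter reads the ship's current weapon, if valid, and also reports whether its ammo is infinite.
; Points come from BP_AstroidsGameMode, with each getter relying on a cast to reach its source.
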(fn GetShipStrengthinPrec
  (bind _asbp_space_ship (Utilities|Casting|CastToBP_SpaceShip (Game|Player|GetPlayerPawn 0)))
  (return (Math|Conversions|ToFloat(Integer) (Math|Float|Round (Math|Float|MapRangeClamped (Class|ForceFieldComponent|GetCurrentForceFieldStrength (Variables|/Game/Blueprints/BP_SpaceShip.BP_SpaceShip_C|GetForceField_Ref _asbp_space_ship)) (Class|ForceFieldComponent|GetForceFieldStrength (Variables|/Game/Blueprints/BP_SpaceShip.BP_SpaceShip_C|GetForceField_Ref _asbp_space_ship)) 0.0 1e+02 0.0)))))

(fn GetCurrentWeaponAmmunition
  (bind _asbp_space_ship (Utilities|Casting|CastToBP_SpaceShip (Game|Player|GetPlayerPawn 0)))
  (Utilities|IsValid (Variables|/Script/ProgTestAstroids.SpaceShip|GetCurrentWeapon _asbp_space_ship)
    (:Is%20Valid
      (return (Variables|/Script/ProgTestAstroids.Weapon|GetAmmunition (Variables|/Script/ProgTestAstroids.SpaceShip|GetCurrentWeapon _asbp_space_ship)) (Variables|/Script/ProgTestAstroids.Weapon|GetisInfinitAmmunition (Variables|/Script/ProgTestAstroids.SpaceShip|GetCurrentWeapon _asbp_space_ship))))))

(fn GetPoints
  (bind _asbp_astroids_game_mode (Utilities|Casting|CastToBP_AstroidsGameMode (Game|GetGameMode)))
  (return (Variables|/Script/ProgTestAstroids.AstroidsGameMode|GetPoints _asbp_astroids_game_mode)))