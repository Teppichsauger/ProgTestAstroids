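; BP_Weapon_V2 is a weapon variant that fires projectiles from up to two muzzles at once.
; It overrides StartFire, runs the parent logic, then calls FireWeapon at the world location of each valid muzzle component.
; Both shots use BP_Projectile with the same hardcoded damage, and the construction script only defers to the parent.
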(event EventStartFire
  (bind _muzzle (Variables|Default|GetMuzzle))
  (bind _muzzle1 (Variables|Default|GetMuzzle1))
  (|CallParentFunction)
  (Utilities|IsValid _muzzle
    (:Is%20Valid
      (Class|Weapon|FireWeapon (Transformation|GetWorldLocation _muzzle) 15.0 "/Game/Blueprints/Weapons/BP_Projectile.BP_Projectile_C"))
    (:Is%20Not%20Valid
      _))
  (Utilities|IsValid _muzzle1
    (:Is%20Valid
      (Class|Weapon|FireWeapon (Transformation|GetWorldLocation _muzzle1) 15.0 "/Game/Blueprints/Weapons/BP_Projectile.BP_Projectile_C"))))

(fn ConstructionScript
  (|CallParentFunction))