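; BP_Weapon_V3 is a multi-muzzle weapon variant that fires a projectile from up to four muzzles at once.
; On StartFire, it validity-checks each muzzle component and calls FireWeapon at that muzzle's world location.
; Every shot uses BP_Projectile with the same hard-coded damage, and the construction script only calls its parent.
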(event EventStartFire
  (bind _muzzle (Variables|Default|GetMuzzle))
  (bind _muzzle1 (Variables|Default|GetMuzzle1))
  (bind _muzzle3 (Variables|Default|GetMuzzle3))
  (bind _muzzle4 (Variables|Default|GetMuzzle4))
  (Utilities|IsValid _muzzle
    (:Is%20Valid
      (Class|Weapon|FireWeapon (Transformation|GetWorldLocation _muzzle) 2e+01 "/Game/Blueprints/Weapons/BP_Projectile.BP_Projectile_C"))
    (:Is%20Not%20Valid
      _))
  (Utilities|IsValid _muzzle1
    (:Is%20Valid
      (Class|Weapon|FireWeapon (Transformation|GetWorldLocation _muzzle1) 2e+01 "/Game/Blueprints/Weapons/BP_Projectile.BP_Projectile_C"))
    (:Is%20Not%20Valid
      _))
  (Utilities|IsValid _muzzle3
    (:Is%20Valid
      (Class|Weapon|FireWeapon (Transformation|GetWorldLocation _muzzle3) 2e+01 "/Game/Blueprints/Weapons/BP_Projectile.BP_Projectile_C"))
    (:Is%20Not%20Valid
      _))
  (Utilities|IsValid _muzzle4
    (:Is%20Valid
      (Class|Weapon|FireWeapon (Transformation|GetWorldLocation _muzzle4) 2e+01 "/Game/Blueprints/Weapons/BP_Projectile.BP_Projectile_C"))))

(fn ConstructionScript
  (|CallParentFunction))