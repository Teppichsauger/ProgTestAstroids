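; Player spaceship Blueprint that handles the ship's game-over crash sequence and caches its ForceField reference at BeginPlay.
; GameOverEvent spawns an explosion, disables player input and picks a direction from the sign of the ship's Y position.
; A slowed timeline lerps the ship from its current transform toward the opposite side with a roll.
; In parallel, a short delay reloads the current level.
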(event EventBeginPlay
  (|CallParentFunction)
  (Variables|Default|SetForceField_Ref (Variables|Default|GetForceField)))

(event EventGameOverEvent
  (bind _self self)
  (bind _returnvalue (Transformation|GetActorRotation _self))
  (bind (_roll _pitch _yaw) (Math|Rotator|BreakRotator _returnvalue))
  (CallFunction|SetDirection)
  (Effects|SpawnEmitteratLocation "/Game/StarterContent/Particles/P_Explosion.P_Explosion" (Transformation|GetActorLocation self))
  (Utilities|FlowControl|Sequence
    (:then_0
      (Input|DisableInput (Game|Player|GetPlayerPawn 0) (Game|GetPlayerController 0))
      (Components|Timeline|SetPlayRate (Variables|Default|GetGameOverAnim) 0.01)
      (bind _alpha (Timeline|GameOverAnim Play)
        (:Update
          (Transformation|SetActorLocation self (Math|Vector|Lerp(Vector) (Transformation|GetActorLocation self) (Utilities|Select :Index (Variables|Default|GetDirection) :Option%200 "450.000000,800.000000, 0" :Option%201 "450.000000,-800.000000, 0") _alpha) false false)
          (Transformation|SetActorRotation self (Math|Rotator|Lerp(Rotator) _returnvalue (Utilities|Select :Index (Variables|Default|GetDirection) :Option%200 (Math|Rotator|MakeRotator -4e+01 _pitch _yaw) :Option%201 (Math|Rotator|MakeRotator 4e+01 _pitch _yaw)) _alpha)))))
    (:then_1
      (Utilities|FlowControl|Delay 4.0)
      (bind _returnvalue_2 (Game|GetCurrentLevelName true))
      (Game|OpenLevel(byName) (Utilities|String|StringToName _returnvalue_2)))))

(fn ConstructionScript)

(fn SetDirection
  (if (< (.y (Transformation|GetActorLocation self)) 0.0)
    (Variables|Default|SetDirection 0)
    (else
      (Variables|Default|SetDirection 1))))